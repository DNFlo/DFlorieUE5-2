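; Interactable door that swings open when interacted with while unlocked, then closes itself after a short delay.
; A dot product of the door's forward vector and the direction to the player picks the swing direction.
; A Timeline lerps the Arrow component's yaw and plays in reverse to close.
; The construction script tints the Cube through a dynamic material instance using PickupColor.
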(event `/Game/Interfaces/Interface_Interact.INT_interact`
  (params (PlayerRef :type "/Game/Player/BP_PlayerChar Object Reference"))
  ; Door Interaction
  (if (`self.isUnlocked`)
    (bind _returnvalue (`self.UpdateDoorAngle`))
    (bind (_direction _alpha) (`Timeline|Timeline` :!label _label)
      (:`Update`
        (`SceneComponent.K2_SetRelativeRotation` (`self.Arrow`) (`KismetMathLibrary.MakeRotator` 0.0 0.0 (`KismetMathLibrary.Lerp` 0.0 _returnvalue _alpha)) false false))
      (:`Finished`
        (`KismetSystemLibrary.Delay` 2.0)
        (`self.ReverseTimeline`)))))

(event `ReverseTimeline`
  ; Door Interaction
  (goto _label :!via `Reverse`))

(fn `UpdateDoorAngle`
  (returns (ReturnValue :type "Float (double-precision)"))
  (return (select `bool` (> (`KismetMathLibrary.Dot_VectorVector` (`KismetMathLibrary.GetDirectionUnitVector` (`self.K2_GetActorLocation`) (`self.K2_GetActorLocation` (`GameplayStatics.GetPlayerCharacter` 0))) (`self.GetActorForwardVector`)) 0.0) :`false` -90.0 :`true` 90.0)))

(fn `UserConstructionScript`
  (bind _returnvalue (`PrimitiveComponent.CreateDynamicMaterialInstance` (`self.Cube`) 0 "/Game/Interactibles/AnimatedInteractibles/MAT_Color.MAT_Color" "None"))
  (bind _output_get (set `self.ColorDMI` _returnvalue))
  (`MaterialInstanceDynamic.SetVectorParameterValue` _output_get "Color" (`self.PickupColor`)))